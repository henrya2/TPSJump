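; BP_GameManager procedurally builds an endlessly rising trail of BP_JumpPad actors.
; BeginPlay spawns five pads, then a one-second looping timer re-enters the same spawn logic.
; Each pad is offset from the previous one by a random signed XY distance beyond a minimum, with height growing with the running count.
; Once the count exceeds the maximum, the oldest pad in the tracked array is destroyed, keeping a moving window.
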(event Custom|CustomEvent_0
  (bind _returnvalue (Math|Random|RandomFloatinRange 5e+01 2e+02))
  (bind _mindistance (Variables|Default|GetMinDistance))
  (bind _mindistance_2 (Variables|Default|GetMinDistance))
  (bind _returnvalue_2 (+ _mindistance _returnvalue))
  (bind _returnvalue_3 (Game|SpawnActorfromClass "/Game/Blueprints/BP_JumpPad.BP_JumpPad_C" (Math|Transform|MakeTransform "0, 0, 0") true 0 0))
  (Utilities|IsValid (Variables|Default|GetPrevJumpPadActor)
    (:Is%20Valid
      (if (Math|Random|RandomBool)
        (Variables|Default|SetTmpDeltaXSign 1.0)
        (else
          (Variables|Default|SetTmpDeltaXSign -1.0)))
      (if (Math|Random|RandomBool)
        (Variables|Default|SetTmpDeltaYSign 1.0)
        (else
          (Variables|Default|SetTmpDeltaYSign -1.0)))
      (Transformation|SetActorLocation _returnvalue_3 (Math|Vector|MakeVector (+ (* (+ (Math|Random|RandomFloatinRange 5e+01 1.8e+02) _mindistance_2) (Variables|Default|GetTmpDeltaXSign)) (.x (Transformation|GetActorLocation (Variables|Default|GetPrevJumpPadActor)))) (+ (* (+ (Math|Random|RandomFloatinRange 5e+01 1.8e+02) _mindistance_2) (Variables|Default|GetTmpDeltaYSign)) (.y (Transformation|GetActorLocation (Variables|Default|GetPrevJumpPadActor)))) (+ (* (Variables|Default|GetJumpPadCount) (Variables|Default|GetPadHeight)) (Variables|Default|GetStartHeight))) false))
    (:Is%20Not%20Valid
      (if (Math|Random|RandomBool)
        (Variables|Default|SetTmpDeltaXSign 1.0)
        (else
          (Variables|Default|SetTmpDeltaXSign -1.0)))
      (if (Math|Random|RandomBool)
        (bind _output_get (Variables|Default|SetTmpDeltaYSign 1.0))
        (else
          (bind _output_get_2 (Variables|Default|SetTmpDeltaYSign -1.0))))
      (Transformation|SetActorLocation _returnvalue_3 (Math|Vector|MakeVector (* _returnvalue_2 _output_get) (* _returnvalue_2 _output_get_2) (+ (* (Variables|Default|GetJumpPadCount) (Variables|Default|GetPadHeight)) (Variables|Default|GetStartHeight))) false)))
  (bind _output_get_3 (Variables|Default|SetPrevJumpPadActor _returnvalue_3))
  (Utilities|Array|Add (Variables|Default|GetJumpPadsArray) _output_get_3)
  (bind _output_get_4 (Variables|Default|SetJumpPadCount (+ (Variables|Default|GetJumpPadCount) 1)))
  (if (> _output_get_4 (Variables|Default|GetMaxPadsCount))
    (Actor|DestroyActor (Utilities|Array|Get(acopy) (Variables|Default|GetJumpPadsArray)))
    (Utilities|Array|RemoveIndex (Variables|Default|GetJumpPadsArray))))

(event EventBeginPlay
  (bind _returnvalue (Math|Random|RandomFloatinRange 5e+01 2e+02))
  (bind _mindistance (Variables|Default|GetMinDistance))
  (bind _mindistance_2 (Variables|Default|GetMinDistance))
  (bind _returnvalue_2 (+ _mindistance _returnvalue))
  (for _index (range 1 5)
    (bind _returnvalue_3 (Game|SpawnActorfromClass "/Game/Blueprints/BP_JumpPad.BP_JumpPad_C" (Math|Transform|MakeTransform "0, 0, 0") true 0 0))
    (Utilities|IsValid (Variables|Default|GetPrevJumpPadActor)
      (:Is%20Valid
        (if (Math|Random|RandomBool)
          (Variables|Default|SetTmpDeltaXSign 1.0)
          (else
            (Variables|Default|SetTmpDeltaXSign -1.0)))
        (if (Math|Random|RandomBool)
          (Variables|Default|SetTmpDeltaYSign 1.0)
          (else
            (Variables|Default|SetTmpDeltaYSign -1.0)))
        (Transformation|SetActorLocation _returnvalue_3 (Math|Vector|MakeVector (+ (* (+ (Math|Random|RandomFloatinRange 5e+01 1.8e+02) _mindistance_2) (Variables|Default|GetTmpDeltaXSign)) (.x (Transformation|GetActorLocation (Variables|Default|GetPrevJumpPadActor)))) (+ (* (+ (Math|Random|RandomFloatinRange 5e+01 1.8e+02) _mindistance_2) (Variables|Default|GetTmpDeltaYSign)) (.y (Transformation|GetActorLocation (Variables|Default|GetPrevJumpPadActor)))) (+ (* (Variables|Default|GetJumpPadCount) (Variables|Default|GetPadHeight)) (Variables|Default|GetStartHeight))) false))
      (:Is%20Not%20Valid
        (if (Math|Random|RandomBool)
          (Variables|Default|SetTmpDeltaXSign 1.0)
          (else
            (Variables|Default|SetTmpDeltaXSign -1.0)))
        (if (Math|Random|RandomBool)
          (bind _output_get (Variables|Default|SetTmpDeltaYSign 1.0))
          (else
            (bind _output_get_2 (Variables|Default|SetTmpDeltaYSign -1.0))))
        (Transformation|SetActorLocation _returnvalue_3 (Math|Vector|MakeVector (* _returnvalue_2 _output_get) (* _returnvalue_2 _output_get_2) (+ (* (Variables|Default|GetJumpPadCount) (Variables|Default|GetPadHeight)) (Variables|Default|GetStartHeight))) false)))
    (bind _output_get_3 (Variables|Default|SetPrevJumpPadActor _returnvalue_3))
    (Utilities|Array|Add (Variables|Default|GetJumpPadsArray) _output_get_3)
    (bind _output_get_4 (Variables|Default|SetJumpPadCount (+ (Variables|Default|GetJumpPadCount) 1)))
    (if (> _output_get_4 (Variables|Default|GetMaxPadsCount))
      (Actor|DestroyActor (Utilities|Array|Get(acopy) (Variables|Default|GetJumpPadsArray)))
      (Utilities|Array|RemoveIndex (Variables|Default|GetJumpPadsArray))))
  (Utilities|Time|SetTimerbyEvent (delegate Custom|CustomEvent_0) 1.0 true))

(event Collision|EventActorBeginOverlap
  (params (OtherActor :type Actor%20Object%20Reference)))

(event EventTick
  (params (DeltaSeconds :type Float%20%28single-precision%29)))

(event EventEndPlay
  (params (EndPlayReason :type EEndPlayReason%20Enum :default "Destroyed"))
  (Class|KismetSystemLibrary|ClearTimerDelegate (delegate Custom|CustomEvent_0)))

(fn ConstructionScript)